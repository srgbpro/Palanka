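; Test trigger zone for a car that runs a staged number-check, quiz and photo interaction.
; Character overlap enables input and shows prompts, while boolean flags and DoOnce gates sequence the E key through a zoomed number view, a mouse-driven quiz menu, then photo mode.
; Each stage blends the view target between cameras and swaps widgets.
; In photo mode, C plays a shutter sound and flash, then restores character view and input.
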(event Custom|ObjectSender
  (params (Camera :type Camera%20Actor%20Object%20Reference))
  ;[1 1 1] Phohozone
)

(event Collision|EventActorBeginOverlap
  (params (OtherActor :type Actor%20Object%20Reference))
  (Utilities|Casting|CastToCharacter OtherActor)
  (Input|EnableInput (Game|GetPlayerController 0))
  (if (Variables|Default|GetFinal)
    (if (Variables|Default|GetPhoto_done)
      (bind _returnvalue (UserInterface|CreateWidget "/Game/OleksiiKaliaka/Blueprints/Check_photo.Check_photo_C"))
      (UserInterface|Viewport|AddtoViewport _returnvalue 0))
    (else
      (bind _returnvalue_2 (UserInterface|CreateWidget "/Game/JuliaKropivnaya/Blueprints/Zoom_number.Zoom_number_C"))
      (UserInterface|Viewport|AddtoViewport _returnvalue_2 0))))

(event Collision|EventActorEndOverlap
  (params (OtherActor :type Actor%20Object%20Reference))
  (Utilities|Casting|CastToCharacter OtherActor)
  (Input|DisableInput (Game|GetPlayerController 0))
  (if (not (Variables|Default|GetFinal))
    (Widget|RemovefromParent (stale Collision|EventActorBeginOverlap _returnvalue_2))))

(event Input|KeyboardEvents|E
  (params (Key :type Key%20Structure))
  (bind _returnvalue (Game|GetPlayerController 0))
  (bind _returnvalue_2 (Game|GetPlayerController 0))
  (:Pressed
    (if (Variables|Default|GetStart)
      (Input|DisableInput (Game|GetPlayerCharacter 0) (Game|GetPlayerController 0))
      (Game|Player|SetViewTargetwithBlend _returnvalue_2 (Components|GetOwner (Variables|Default|GetCamera_for_zoom)) 1.0 "VTBlend_Linear" 0.0 false)
      (Widget|RemovefromParent (stale Collision|EventActorBeginOverlap _returnvalue_2))
      (Utilities|FlowControl|Delay 2.5)
      (Variables|Default|SetStart false)
      (Utilities|FlowControl|DoOnce false
        (:Completed
          (bind _returnvalue_3 (UserInterface|CreateWidget "/Game/JuliaKropivnaya/Blueprints/Check_number.Check_number_C" _returnvalue_2))
          (UserInterface|Viewport|AddtoViewport _returnvalue_3 0)
          (Game|Player|SetViewTargetwithBlend (Game|GetPlayerController 0) (Game|GetPlayerCharacter 0) 1.0 "VTBlend_Linear" 0.0 false)))
      (elif (Variables|Default|GetFinal)
        (Utilities|FlowControl|DoOnce false
          (:Completed
            ;[1 1 1] Phohozone
            (Rendering|SetVisibility (Variables|Default|GetWidget) false false)
            (Game|Player|SetViewTargetwithBlend (Game|GetPlayerController 0) (stale Custom|ObjectSender Camera) 2.0 "VTBlend_Cubic" 0.0 false)
            (Input|DisableInput (Game|GetPlayerCharacter 0) (Game|GetPlayerController 0))
            (bind _returnvalue_4 (UserInterface|CreateWidget "/Game/OleksiiKaliaka/Blueprints/PhotoZone_widget_2.PhotoZone_widget_2_C"))
            (UserInterface|Viewport|AddtoViewport _returnvalue_4 0)
            (bind _returnvalue_5 (UserInterface|CreateWidget "/Game/OleksiiKaliaka/Blueprints/Check_photo.Check_photo_C"))
            (UserInterface|Viewport|AddtoViewport _returnvalue_5 0)
            (Variables|Default|SetPhoto true)))
        (elif (Variables|Default|Get1Camera)
          (Utilities|FlowControl|DoOnce false
            (:Completed
              (Widget|RemovefromParent _returnvalue_3)
              (Components|Activation|Deactivate (Variables|Default|GetCamera_for_zoom))
              (Game|Player|SetViewTargetwithBlend (Game|GetPlayerController 0) (Components|GetOwner (Variables|Default|GetCamera_for_widget)) 1.0 "VTBlend_Linear" 0.0 false)
              (Variables|/Script/Engine.PlayerController|SetbShowMouseCursor _returnvalue true)
              (Variables|/Script/Engine.PlayerController|SetbEnableClickEvents _returnvalue true)
              (bind _returnvalue_6 (UserInterface|CreateWidget "/Game/JuliaKropivnaya/Blueprints/Number_quiz_menu.Number_quiz_menu_C"))
              (UserInterface|Viewport|AddtoViewport _returnvalue_6 0)
              (Variables|Default|Set1Camera false)
              (Variables|Default|SetFinal true)
              (Variables|Default|SetPhoto_done true)
              (Rendering|SetVisibility (Variables|Default|GetWidget) true false))))))))

(event Input|KeyboardEvents|C
  (params (Key :type Key%20Structure))
  (bind _returnvalue (Game|GetPlayerController 0))
  ;[1 1 1] Phohozone
  (:Pressed
    (if (Variables|Default|GetPhoto)
      (Utilities|FlowControl|DoOnce false
        (:Completed
          (Audio|PlaySoundatLocation "/Game/OleksiiKaliaka/Sounds/camera.camera" "0, 0, 0" "0, 0, 0" 1.0 1.0 0.0 0 0 0)
          (bind _returnvalue_2 (UserInterface|CreateWidget "/Game/OleksiiKaliaka/Blueprints/CameraFlash_widget.CameraFlash_widget_C"))
          (UserInterface|Viewport|AddtoViewport _returnvalue_2 0)
          (Widget|RemovefromParent (stale Input|KeyboardEvents|E _returnvalue_4))
          (Widget|RemovefromParent (stale Input|KeyboardEvents|E _returnvalue_5))
          (bind _returnvalue_3 (UserInterface|CreateWidget "/Game/OleksiiKaliaka/Blueprints/PhotoZone_widget_3.PhotoZone_widget_3_C"))
          (UserInterface|Viewport|AddtoViewport _returnvalue_3 0)
          (Utilities|FlowControl|Delay 2.0)
          (Widget|RemovefromParent _returnvalue_3)
          (bind _outactors (Actor|GetAllActorsOfClass "/Script/Engine.Character"))
          (for _array_element _outactors
            (bind _ascharacter (Utilities|Casting|CastToCharacter _array_element))
            (Game|Player|SetViewTargetwithBlend _returnvalue _ascharacter 1.0 "VTBlend_Linear" 0.0 false)
            (Input|EnableInput (Game|GetPlayerCharacter 0) _returnvalue)
            (Variables|Default|SetPhoto_done false)))))))

(fn ConstructionScript)