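; Control panel Blueprint that the player activates with E to play a Matinee sequence and switch two monitor Blueprints.
; Overlapping the panel enables player input and turns on custom depth rendering on its mesh as a highlight.
; Pressing E plays the Matinee, then casts the left and right monitors and sends each a false parameter.
; A controlMatineeSender event declares the Matinee and monitor inputs but has no logic wired to it.
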(event Custom|controlMatineeSender
  (params (MatineeActor :type Matinee%20Actor%20Object%20Reference) (Monitor_left :type Actor%20Object%20Reference) (Monitor_right :type Actor%20Object%20Reference)))

(event Collision|EventActorBeginOverlap
  (params (OtherActor :type Actor%20Object%20Reference))
  ;[1 1 1] Object backlight
  (Input|EnableInput (Game|GetPlayerController 0))
  (Rendering|SetRenderCustomDepth (Variables|/Script/Engine.StaticMeshActor|GetStaticMeshComponent self) true))

(event Input|KeyboardEvents|E
  (params (Key :type Key%20Structure))
  (:Pressed
    (Audio|Components|Audio|Play (stale Custom|controlMatineeSender MatineeActor))
    (bind _asr_monitor_blueprint_2_blueprint (Utilities|Casting|CastTor_monitor_Blueprint2_Blueprint (stale Custom|controlMatineeSender Monitor_left)))
    (Default|ParSenderLeft _asr_monitor_blueprint_2_blueprint false)
    (bind _asr_monitor_blueprint (Utilities|Casting|CastTor_monitor_Blueprint (stale Custom|controlMatineeSender Monitor_right)))
    (Default|ParSenderRight _asr_monitor_blueprint false)))

(fn ConstructionScript)