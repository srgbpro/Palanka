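; Interactive left monitor for a Rapiscan scanner that the player can view up close.
; Par_Sender_Left receives the camera, a flag and the right monitor, swaps the screen material, shows the prompt widget and custom-depth highlight, and enables input.
; After any overlap, E blends to the camera, shows tips, locks character input and triggers the right monitor, or prints a start-the-Rapiscan warning.
; Q removes tips and restores character view and input.
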(event Custom|Par_Sender_Left
  (params (Camera :type Camera%20Actor%20Object%20Reference) (NewParam :type Boolean) (Right_Monitor :type Actor%20Object%20Reference))
  (Class|WidgetComponent|SetTintColorandOpacity (Variables|Default|GetWidget) "(R=1.000000,G=1.000000,B=1.000000,A=1.000000)")
  (Rendering|Material|SetMaterial (Variables|Default|GetStaticMeshComponent) 1 "/Game/OleksiiKaliaka/Meshes/h_rapiscan/h_rapiscan_mat/r_monitor_screen1_01_left.r_monitor_screen1_01_left")
  ;[1 1 1] Object backlight
  (Input|EnableInput (Game|GetPlayerController 0))
  (Rendering|SetRenderCustomDepth (Variables|/Script/Engine.StaticMeshActor|GetStaticMeshComponent self) true))

(event Collision|EventActorBeginOverlap
  (params (OtherActor :type Actor%20Object%20Reference))
  (bind _output_get (Variables|Default|SetoverlapCondition true)))

(event Input|KeyboardEvents|E
  (params (Key :type Key%20Structure))
  (:Pressed
    (if (stale Collision|EventActorBeginOverlap _output_get)
      (if (stale Custom|Par_Sender_Left NewParam)
        (Class|WidgetComponent|SetTintColorandOpacity (Variables|Default|GetWidget) "(R=1.000000,G=1.000000,B=1.000000,A=0.000000)")
        ;[1 1 1] Changing camera position
        (Game|Player|SetViewTargetwithBlend (Game|GetPlayerController 0) (stale Custom|Par_Sender_Left Camera) 3.0 "VTBlend_Linear" 0.0 false)
        ;[1 1 1] Widget
        (bind _returnvalue (UserInterface|CreateWidget "/Game/OleksiiKaliaka/Blueprints/User_tips_2.User_tips_2_C" (Game|GetPlayerController 0)))
        (UserInterface|Viewport|AddtoViewport _returnvalue 0)
        (Rendering|SetRenderCustomDepth (Variables|/Script/Engine.StaticMeshActor|GetStaticMeshComponent self) false)
        (Input|DisableInput (Game|GetPlayerCharacter 0) (Game|GetPlayerController 0))
        (bind _asr_monitor_blueprint (Utilities|Casting|CastTor_monitor_Blueprint (stale Custom|Par_Sender_Left Right_Monitor)))
        (Default|TriggerSender _asr_monitor_blueprint)
        (else
          (Development|PrintString "Запусти рапискан!"))))))

(event Input|KeyboardEvents|Q
  (params (Key :type Key%20Structure))
  ;[1 1 1] return of the camera
  (:Pressed
    (Widget|RemovefromParent (stale Input|KeyboardEvents|E _returnvalue))
    (bind _outactors (Actor|GetAllActorsOfClass "/Script/Engine.Character"))
    (for _array_element _outactors
      (bind _ascharacter (Utilities|Casting|CastToCharacter _array_element))
      (Game|Player|SetViewTargetwithBlend (Game|GetPlayerController 0) _ascharacter 3.0 "VTBlend_Linear" 0.0 false)
      (Input|EnableInput (Game|GetPlayerCharacter 0) (Game|GetPlayerController 0)))))

(fn ConstructionScript
  (|CallParentFunction))