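; Interactive seal exhibit that accepts player input while a Character overlaps it and offers staged camera views.
; With EnterTrigger set, E uses two flags to step through zoom, macro and side cameras, swapping tip and seal widgets.
; The zoom step hides the prompt widget and disables character input.
; Q blends back to the character, restores input, removes zoom-step widgets and clears EnterTrigger, which this graph never sets true.
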(event Custom|ObjectSender
  (params (Zoom_Camera :type Camera%20Actor%20Object%20Reference) (Macro_Camera :type Camera%20Actor%20Object%20Reference) (Side_Camera :type Camera%20Actor%20Object%20Reference)))

(event Collision|EventActorBeginOverlap
  (params (OtherActor :type Actor%20Object%20Reference))
  (Utilities|Casting|CastToCharacter OtherActor)
  (Input|EnableInput (Game|GetPlayerController 0)))

(event Collision|EventActorEndOverlap
  (params (OtherActor :type Actor%20Object%20Reference))
  (Utilities|Casting|CastToCharacter OtherActor)
  (Input|DisableInput (Game|GetPlayerController 0)))

(event Input|KeyboardEvents|E
  (params (Key :type Key%20Structure))
  (bind _returnvalue (Game|GetPlayerController 0))
  (:Pressed
    (if (Variables|Default|GetEnterTrigger)
      (if (Variables|Default|GetTrigger2)
        (Game|Player|SetViewTargetwithBlend (Game|GetPlayerController 0) (stale Custom|ObjectSender Side_Camera) 1.5 "VTBlend_Linear" 0.0 false)
        (elif (Variables|Default|GetTrigger1)
          (Widget|RemovefromParent (stale _returnvalue_4))
          ;[1 1 1] Widget
          (bind _returnvalue_2 (UserInterface|CreateWidget "/Game/OleksiiKaliaka/Blueprints/User_tips_2.User_tips_2_C" (Game|GetPlayerController 0)))
          (UserInterface|Viewport|AddtoViewport _returnvalue_2 0)
          (Game|Player|SetViewTargetwithBlend _returnvalue (stale Custom|ObjectSender Zoom_Camera) 1.5 "VTBlend_Linear" 0.0 false)
          (Class|WidgetComponent|SetTintColorandOpacity (Variables|Default|GetWidget) "(R=0.000000,G=0.000000,B=0.000000,A=0.000000)")
          (Input|DisableInput (Game|GetPlayerCharacter 0) (Game|GetPlayerController 0))
          (Class|WidgetComponent|SetTintColorandOpacity (Variables|Default|GetWidget) "(R=0.000000,G=0.000000,B=0.000000,A=0.000000)")
          (bind _returnvalue_3 (UserInterface|CreateWidget "/Game/OleksiiKaliaka/Blueprints/Seal_widget_2.Seal_widget_2_C" (Game|GetPlayerController 0)))
          (UserInterface|Viewport|AddtoViewport _returnvalue_3 0)
          (Variables|Default|SetTrigger1 false)
          (else
            (Widget|RemovefromParent _returnvalue_2)
            (Widget|RemovefromParent _returnvalue_3)
            (Game|Player|SetViewTargetwithBlend _returnvalue (stale Custom|ObjectSender Macro_Camera) 1.5 "VTBlend_Linear" 0.0 false)
            (Variables|Default|SetTrigger1 true)
            (bind _returnvalue_4 (UserInterface|CreateWidget "/Game/OleksiiKaliaka/Blueprints/User_tips_3.User_tips_3_C" (Game|GetPlayerController 0)))
            (UserInterface|Viewport|AddtoViewport _returnvalue_4 0)
            (Variables|Default|SetTrigger2 true)))))))

(event Input|KeyboardEvents|Q
  (params (Key :type Key%20Structure))
  (bind _returnvalue (Game|GetPlayerController 0))
  (:Pressed
    (bind _outactors (Actor|GetAllActorsOfClass "/Script/Engine.Character"))
    (for _array_element _outactors
      (bind _ascharacter (Utilities|Casting|CastToCharacter _array_element))
      (Game|Player|SetViewTargetwithBlend _returnvalue _ascharacter 3.0 "VTBlend_Linear" 0.0 false)
      (Input|EnableInput (Game|GetPlayerCharacter 0) _returnvalue)
      (Widget|RemovefromParent (stale Input|KeyboardEvents|E _returnvalue_2))
      (Widget|RemovefromParent (stale Input|KeyboardEvents|E _returnvalue_3))
      (Variables|Default|SetEnterTrigger false))))

(fn ConstructionScript)