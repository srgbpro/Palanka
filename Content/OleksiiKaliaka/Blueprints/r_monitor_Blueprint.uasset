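; Interactive monitor Blueprint that changes its screen and toggles an object highlight in response to two events.
; Par_Sender_Right swaps the screen material slot to the "right" screen material, enables player input and turns on Render Custom Depth as a backlight, without reading its Result parameter.
; TriggerSender turns the backlight off but also calls EnableInput, so input is never disabled here.
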(event Custom|Par_Sender_Right
  (params (Result :type Boolean))
  (Rendering|Material|SetMaterial (Variables|Debug|GetStaticMeshComponent) 1 "/Game/OleksiiKaliaka/Meshes/h_rapiscan/h_rapiscan_mat/r_monitor_screen1_01_right.r_monitor_screen1_01_right")
  ;[1 1 1] Object backlight
  (Input|EnableInput (Game|GetPlayerController 0))
  (Rendering|SetRenderCustomDepth (Variables|/Script/Engine.StaticMeshActor|GetStaticMeshComponent self) true))

(event Custom|TriggerSender
  ;[1 1 1] Object backlight off
  (Input|EnableInput (Game|GetPlayerController 0))
  (Rendering|SetRenderCustomDepth (Variables|/Script/Engine.StaticMeshActor|GetStaticMeshComponent self) false))

(fn ConstructionScript)