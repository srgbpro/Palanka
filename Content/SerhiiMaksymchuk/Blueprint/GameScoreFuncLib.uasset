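; Blueprint function library with score helpers for the game.
; PlusScoreForSuccessOperation adds points to a by-reference counter only when an operation succeeds without detection, and returns the counter.
; EvaluateScoreInPercents turns a score and its maximum possible value into a percentage string, using float division and a percent suffix.
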(fn PlusScoreforSuccessOperation
  (params (IsNotDetected :type Boolean) (IsOperationSuccess :type Boolean) (RefCounter :type Integer%20%28by%20ref%29) (PlusScore :type Integer))
  (if IsNotDetected
    (if IsOperationSuccess
      (|SetBy-RefVar RefCounter (+ RefCounter PlusScore))
      (return RefCounter)
      (else
        (return RefCounter)))
    (else
      (return RefCounter))))

(fn EvaluateScoreinPercents
  (params (Score :type Integer) (MaxPossibleScore :type Integer))
  (return (Utilities|String|Append (Utilities|String|ToString(Float) (* 100 (/ (Math|Conversions|ToFloat(Integer) Score) (Math|Conversions|ToFloat(Integer) MaxPossibleScore)))) "%")))