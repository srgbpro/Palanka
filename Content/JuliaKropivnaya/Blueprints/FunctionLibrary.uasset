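; Blueprint function library that supplies random car numbers to the game.
; GetCarNumber returns a random entry from a list of car numbers, while GetCorrectNumber does the same from a separate list of correct car numbers.
; Both draw a random index across the full list on each call, with no tracking of earlier picks, so results can repeat.
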(fn GetCarNumber
  (bind _list_of_car_numbers (LocalVariables|GetList_of_car_numbers))
  (return (Utilities|Array|Get(acopy) _list_of_car_numbers (Math|Random|RandomIntegerinRange 0 (Utilities|Array|LastIndex _list_of_car_numbers)))))

(fn GetCorrectNumber
  (bind _list_of_correct_car_numbers (LocalVariables|GetList_of_correct_car_numbers))
  (return (Utilities|Array|Get(acopy) _list_of_correct_car_numbers (Math|Random|RandomIntegerinRange 0 (Utilities|Array|LastIndex _list_of_correct_car_numbers)))))