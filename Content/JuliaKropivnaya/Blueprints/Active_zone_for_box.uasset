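; Trigger zone for a box quiz that stages camera views and UI when the player presses E inside it.
; Overlap shows a one-time Zoom_number prompt and enables input; leaving removes all widgets and disables input.
; The first press blends to a zoom camera, then after a delay shows Check_number and returns to the character.
; A later press, gated by flags and DoOnce, blends to the widget camera and displays an existing Box_quiz_menu.
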(event OnComponentBeginOverlap(Box)
  (params (OverlappedComponent :type Primitive%20Component%20Object%20Reference) (OtherActor :type Actor%20Object%20Reference) (OtherComp :type Primitive%20Component%20Object%20Reference) (OtherBodyIndex :type Integer) (bFromSweep :type Boolean) (SweepResult :type Hit%20Result%20Structure%20%28by%20ref%29))
  (Utilities|FlowControl|DoOnce false
    (:Completed
      (bind _returnvalue (UserInterface|CreateWidget "/Game/JuliaKropivnaya/Blueprints/Zoom_number.Zoom_number_C"))
      (UserInterface|Viewport|AddtoViewport _returnvalue 0)
      (Input|EnableInput (Game|GetPlayerController 0)))))

(event OnComponentEndOverlap(Box)
  (params (OverlappedComponent :type Primitive%20Component%20Object%20Reference) (OtherActor :type Actor%20Object%20Reference) (OtherComp :type Primitive%20Component%20Object%20Reference) (OtherBodyIndex :type Integer))
  (bind _returnvalue (Game|GetPlayerController 0))
  (Viewport|RemoveAllWidgets)
  (Input|DisableInput (Game|GetPlayerController 0))
  (Variables|/Script/Engine.PlayerController|SetbShowMouseCursor _returnvalue false)
  (Variables|/Script/Engine.PlayerController|SetbEnableClickEvents _returnvalue false))

(event Input|KeyboardEvents|E
  (params (Key :type Key%20Structure))
  (bind _returnvalue (Game|GetPlayerController 0))
  (bind _camera_for_zoom (Variables|Default|GetCamera_for_zoom))
  (:Pressed
    (if (Variables|Default|GetStart)
      (Game|Player|SetViewTargetwithBlend _returnvalue (Components|GetOwner _camera_for_zoom) 1.0 "VTBlend_Linear" 0.0 false)
      (Variables|/Script/Engine.PlayerController|SetbShowMouseCursor _returnvalue true)
      (Variables|/Script/Engine.PlayerController|SetbEnableClickEvents _returnvalue true)
      (Utilities|FlowControl|Delay 2.0)
      (Variables|Default|SetStart false)
      (Utilities|FlowControl|DoOnce false
        (:Completed
          (bind _returnvalue_2 (UserInterface|CreateWidget "/Game/JuliaKropivnaya/Blueprints/Check_number.Check_number_C" _returnvalue))
          (UserInterface|Viewport|AddtoViewport _returnvalue_2 0)
          (Widget|RemovefromParent (stale OnComponentBeginOverlap(Box) _returnvalue))
          (Game|Player|SetViewTargetwithBlend _returnvalue (Game|GetPlayerCharacter 0) 1.0 "VTBlend_Linear" 0.0 false)))
      (elif (Variables|Default|Get1Camera)
        (Utilities|FlowControl|DoOnce false
          (:Completed
            (Widget|RemovefromParent _returnvalue_2)
            (Components|Activation|Deactivate _camera_for_zoom)
            (Game|Player|SetViewTargetwithBlend (Game|GetPlayerController 0) (Components|GetOwner (Variables|Default|GetCamera_for_widget)) 2.0 "VTBlend_Linear" 0.0 false)
            (Utilities|FlowControl|Delay 2.0)
            (bind _foundwidgets (Widget|GetAllWidgetsOfClass "/Game/JuliaKropivnaya/Blueprints/Box_quiz_menu.Box_quiz_menu_C" false))
            (UserInterface|Viewport|AddtoViewport (Utilities|Array|Get(acopy) _foundwidgets) 0)
            (Variables|Default|Set1Camera false)))))))

(fn ConstructionScript)