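; BP_GameInstanceF is a game instance Blueprint that switches between the gameplay level and the multiplayer main menu.
; Its two events, LoadGameLevel and LoadMainMenu, each clear all widgets, show a WB_LoadingScreen and open a hard-coded level by name.
; The loading screen sits on a fixed short Delay before the level opens, so it does not track actual load progress.
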(event Custom|LoadGameLevel
  (Viewport|RemoveAllWidgets)
  (bind _returnvalue (UserInterface|CreateWidget "/Game/Blueprints/Widgets/WB_LoadingScreen.WB_LoadingScreen_C"))
  (UserInterface|Viewport|AddtoViewport _returnvalue 0)
  (Utilities|FlowControl|Delay 2.0)
  (Game|OpenLevel(byName) "palanka_test_v2_03"))

(event Custom|LoadMainMenu
  (Viewport|RemoveAllWidgets)
  (bind _returnvalue (UserInterface|CreateWidget "/Game/Blueprints/Widgets/WB_LoadingScreen.WB_LoadingScreen_C"))
  (UserInterface|Viewport|AddtoViewport _returnvalue 0)
  (Utilities|FlowControl|Delay 2.0)
  (Game|OpenLevel(byName) "MainMenu_MP"))