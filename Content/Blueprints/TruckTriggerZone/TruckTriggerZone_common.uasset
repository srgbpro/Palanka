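; TruckTriggerZone is a trigger zone that lets the player hide and unhide a tent while a Character overlaps it.
; Overlap begin and end enable and disable player input, with H and G toggling the tent root's visibility and collision.
; A TentHide flag gates each key and selects the on-screen prompt from a newly created notification widget.
; The tent reference is intended to come from the level Blueprint.
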(event Custom|ObjectSender
  (params (Tent :type Actor%20Object%20Reference))
  ;[1 1 1] Get reference to tent from level BP
)

(event Custom|ReturnValue)

(event Collision|EventActorBeginOverlap
  (params (OtherActor :type Actor%20Object%20Reference))
  (Utilities|Casting|CastToCharacter OtherActor)
  (Input|EnableInput (Game|GetPlayerController 0))
  (CallFunction|ShowNotification))

(event Collision|EventActorEndOverlap
  (params (OtherActor :type Actor%20Object%20Reference))
  (Utilities|Casting|CastToCharacter OtherActor)
  (Input|DisableInput (Game|GetPlayerController 0)))

(event Input|KeyboardEvents|H
  (params (Key :type Key%20Structure))
  ;[1 1 1] Hide tent
  (:Pressed
    (if (not (Variables|Default|GetTentHide))
      (Rendering|ToggleVisibility (Variables|/Script/Engine.Actor|GetRootComponent (stale Custom|ObjectSender Tent)) false)
      (Variables|Default|SetTentHide true)
      (CallFunction|ShowNotification)
      ;[1 1 1] Collision manipulation
      (bind _asstatic_mesh_component (Utilities|Casting|CastToStaticMeshComponent (Variables|/Script/Engine.Actor|GetRootComponent (stale Custom|ObjectSender Tent))))
      (Collision|SetCollisionEnabled _asstatic_mesh_component "NoCollision"))))

(event Input|KeyboardEvents|G
  (params (Key :type Key%20Structure))
  ;[1 1 1] Show tent
  (:Pressed
    (if (Variables|Default|GetTentHide)
      (Rendering|ToggleVisibility (Variables|/Script/Engine.Actor|GetRootComponent (stale Custom|ObjectSender Tent)) false)
      (Variables|Default|SetTentHide false)
      (CallFunction|ShowNotification)
      ;[1 1 1] Collision manipulation
      (bind _asstatic_mesh_component (Utilities|Casting|CastToStaticMeshComponent (Variables|/Script/Engine.Actor|GetRootComponent (stale Custom|ObjectSender Tent))))
      (Collision|SetCollisionEnabled _asstatic_mesh_component "QueryAndPhysics"))))

(fn ConstructionScript)

(fn ShowNotification
  (bind _returnvalue (UserInterface|CreateWidget "/Game/Widgets/InformationNotificationWidget_Common.InformationNotificationWidget_Common_C"))
  (if (not (Variables|Default|GetTentHide))
    (Variables|/Game/Widgets/InformationNotificationWidget_Common.InformationNotificationWidget_Common_C|SetMessageLine1 _returnvalue "Press 'h' to")
    (Variables|/Game/Widgets/InformationNotificationWidget_Common.InformationNotificationWidget_Common_C|SetMessageLine2 _returnvalue "hide tent")
    (else
      (Variables|/Game/Widgets/InformationNotificationWidget_Common.InformationNotificationWidget_Common_C|SetMessageLine1 _returnvalue "Press 'g' to")
      (Variables|/Game/Widgets/InformationNotificationWidget_Common.InformationNotificationWidget_Common_C|SetMessageLine2 _returnvalue "unhide tent")))
  (UserInterface|Viewport|AddtoViewport _returnvalue 0))