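; Blueprint for a Rapiscan monitor that shows a left-screen material and a highlight on its static mesh.
; Par_Sender_Left swaps the screen material slot to the left-screen material and turns on custom depth rendering as an object backlight.
; TriggerSender turns that backlight off and leaves the material as it is.
; Both events enable input for the first player controller, and neither uses any parameters it receives.
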(event Custom|Par_Sender_Left
  (params (Camera :type Camera%20Actor%20Object%20Reference) (NewParam :type Boolean) (Right_Monitor :type Actor%20Object%20Reference))
  (Rendering|Material|SetMaterial (Variables|Default|GetStaticMeshComponent) 1 "/Game/Materials/mat_rapiscan/mat_r_monitor_screen_left.mat_r_monitor_screen_left")
  ;[1 1 1] Object backlight
  (Input|EnableInput (Game|GetPlayerController 0))
  (Rendering|SetRenderCustomDepth (Variables|/Script/Engine.StaticMeshActor|GetStaticMeshComponent self) true))

(event Custom|TriggerSender
  ;[1 1 1] Object backlight off
  (Input|EnableInput (Game|GetPlayerController 0))
  (Rendering|SetRenderCustomDepth (Variables|/Script/Engine.StaticMeshActor|GetStaticMeshComponent self) false))

(fn ConstructionScript
  (|CallParentFunction))