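; Photo zone actor that lets the player step into a staged camera shot and take a picture, usable only once.
; Overlapping characters toggle the actor's input; E blends to the photo camera, locks player movement, hides the prompt widget and shows photo UI.
; C plays a shutter sound and flash, then swaps UI; Q blends back to the character and restores input.
; Two booleans gate the stages, and the completion flag never resets.
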(event Custom|ObjectSender
  (params (Camera :type Camera%20Actor%20Object%20Reference)))

(event Collision|EventActorBeginOverlap
  (params (OtherActor :type Actor%20Object%20Reference))
  (Utilities|Casting|CastToCharacter OtherActor)
  (Input|EnableInput (Game|GetPlayerController 0)))

(event Collision|EventActorEndOverlap
  (params (OtherActor :type Actor%20Object%20Reference))
  (Utilities|Casting|CastToCharacter OtherActor)
  (Input|DisableInput (Game|GetPlayerController 0)))

(event Input|KeyboardEvents|E
  (params (Key :type Key%20Structure))
  (:Pressed
    (if (not (Variables|Default|GetCondition_2))
      (if (not (Variables|Default|GetCondition))
        ;[1 1 1] Changing camera position
        (Game|Player|SetViewTargetwithBlend (Game|GetPlayerController 0) (stale Custom|ObjectSender Camera) 2.0 "VTBlend_Cubic" 0.0 false)
        (Input|DisableInput (Game|GetPlayerCharacter 0) (Game|GetPlayerController 0))
        (Class|WidgetComponent|SetTintColorandOpacity (Variables|Default|GetWidget) "(R=0.000000,G=0.000000,B=0.000000,A=0.000000)")
        (bind _returnvalue (UserInterface|CreateWidget "/Game/Widgets/wdgt_photozone/wdgt_photozone_2.wdgt_photozone_2_C"))
        (UserInterface|Viewport|AddtoViewport _returnvalue 0)
        (Variables|Default|SetCondition true)))))

(event Input|KeyboardEvents|Q
  (params (Key :type Key%20Structure))
  (bind _returnvalue (Game|GetPlayerController 0))
  (:Pressed
    (if (Variables|Default|GetCondition_2)
      (Widget|RemovefromParent (stale Input|KeyboardEvents|C _returnvalue_2))
      (bind _outactors (Actor|GetAllActorsOfClass "/Script/Engine.Character"))
      (for _array_element _outactors
        (bind _ascharacter (Utilities|Casting|CastToCharacter _array_element))
        (Game|Player|SetViewTargetwithBlend _returnvalue _ascharacter 2.0 "VTBlend_Linear" 0.0 false)
        (Input|EnableInput (Game|GetPlayerCharacter 0) _returnvalue)))))

(event Input|KeyboardEvents|C
  (params (Key :type Key%20Structure))
  (:Pressed
    (if (Variables|Default|GetCondition)
      (Audio|PlaySoundatLocation "/Game/OleksiiKaliaka/Sounds/camera.camera" "0, 0, 0" "0, 0, 0" 1.0 1.0 0.0 0 0 0)
      (bind _returnvalue (UserInterface|CreateWidget "/Game/Widgets/wdgt_photozone/wdgt_camera_flash.wdgt_camera_flash_C"))
      (UserInterface|Viewport|AddtoViewport _returnvalue 0)
      (Widget|RemovefromParent (stale Input|KeyboardEvents|E _returnvalue))
      (bind _returnvalue_2 (UserInterface|CreateWidget "/Game/Widgets/wdgt_photozone/wdgt_photozone_3.wdgt_photozone_3_C"))
      (UserInterface|Viewport|AddtoViewport _returnvalue_2 0)
      (Variables|Default|SetCondition_2 true)
      (Variables|Default|SetCondition false))))

(fn ConstructionScript)